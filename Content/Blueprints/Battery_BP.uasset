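; Battery pickup actor that the player collects with E, acting as a key by setting PlayerHasKey on PlayerCharacterBP.
; A collision overlap with the player sets an in-trigger flag and calls EnableInput on that character, and leaving clears the flag.
; Pressing E while the flag is set destroys the battery, sets the key flag on player 0's character and prints a confirmation.
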(event `self.Collision.OnComponentBeginOverlap`
  (params (OverlappedComponent :type "PrimitiveComponent Object Reference") (OtherActor :type "Actor Object Reference") (OtherComp :type "PrimitiveComponent Object Reference") (OtherBodyIndex :type Integer) (bFromSweep :type Boolean) (SweepResult :type "HitResult Structure (by ref)"))
  (bind _asplayer_character_bp (cast `/Game/TopDownBP/Blueprints/PlayerCharacterBP` OtherActor))
  (`self.EnableInput` _asplayer_character_bp null)
  (set `self.IsInTrigger` true))

(event `self.Collision.OnComponentEndOverlap`
  (params (OverlappedComponent :type "PrimitiveComponent Object Reference") (OtherActor :type "Actor Object Reference") (OtherComp :type "PrimitiveComponent Object Reference") (OtherBodyIndex :type Integer))
  (cast `/Game/TopDownBP/Blueprints/PlayerCharacterBP` OtherActor)
  (set `self.IsInTrigger` false))

(event `Key|E` :consume false
  (params (Key :type "Key Structure"))
  (:`Pressed`
    (if (`self.IsInTrigger`)
      (`self.K2_DestroyActor`)
      (bind _asplayer_character_bp (cast `/Game/TopDownBP/Blueprints/PlayerCharacterBP` (`GameplayStatics.GetPlayerCharacter` 0)))
      (set `/Game/TopDownBP/Blueprints/PlayerCharacterBP.PlayerHasKey?` true _asplayer_character_bp)
      (`KismetSystemLibrary.PrintString` "Player Has Key"))))

(fn `UserConstructionScript`)