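; Cupboard actor that highlights itself when the player character overlaps it and can show an E-to-search prompt.
; Overlap begin and end toggle custom depth and stencil on the Cupboard component, presumably for an outline effect.
; The prompt widget is created only if the player has neither a key nor bats in inventory; this graph never removes it.
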(event `self.ReceiveActorBeginOverlap`
  (params (OtherActor :type "Actor Object Reference"))
  (bind _cupboard (`self.Cupboard`))
  (cast `/Game/TopDownBP/Blueprints/PlayerCharacterBP` OtherActor)
  (`PrimitiveComponent.SetRenderCustomDepth` _cupboard true)
  (`PrimitiveComponent.SetCustomDepthStencilValue` _cupboard 2)
  (bind _asplayer_character_bp (cast `/Game/TopDownBP/Blueprints/PlayerCharacterBP` (`GameplayStatics.GetPlayerCharacter` 0)))
  (if (not (or (`/Game/TopDownBP/Blueprints/PlayerCharacterBP.PlayerHasKey?` _asplayer_character_bp) (> (`/Game/TopDownBP/Blueprints/PlayerCharacterBP.BatsInInv` _asplayer_character_bp) 0)))
    (bind _returnvalue (`|CreateWidget` "/Game/UI_Widgets/Pick-up_Widget/EToSearch.EToSearch_C" (`GameplayStatics.GetPlayerController` 0)))
    (`UserWidget.AddToViewport` _returnvalue 0)))

(event `self.ReceiveActorEndOverlap`
  (params (OtherActor :type "Actor Object Reference"))
  (bind _cupboard (`self.Cupboard`))
  (cast `/Game/TopDownBP/Blueprints/PlayerCharacterBP` OtherActor)
  (`PrimitiveComponent.SetRenderCustomDepth` _cupboard false)
  (`PrimitiveComponent.SetCustomDepthStencilValue` _cupboard 0))

(fn `UserConstructionScript`)