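; Empty_BP is an interactable that shows a "nothing here" widget when the player presses Interact nearby.
; Its Collision overlaps set an IsInTrigger flag for PlayerCharacterBP and, on entry, call EnableInput on that character.
; Pressing Interact inside the trigger creates a NothingHere_Widget and adds it to the viewport, with no removal handled in this Blueprint.
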(event `self.Collision.OnComponentBeginOverlap`
  (params (OverlappedComponent :type "PrimitiveComponent Object Reference") (OtherActor :type "Actor Object Reference") (OtherComp :type "PrimitiveComponent Object Reference") (OtherBodyIndex :type Integer) (bFromSweep :type Boolean) (SweepResult :type "HitResult Structure (by ref)"))
  (bind _asplayer_character_bp (cast `/Game/TopDownBP/Blueprints/PlayerCharacterBP` OtherActor))
  (`self.EnableInput` _asplayer_character_bp null)
  (set `self.IsInTrigger` true))

(event `self.Collision.OnComponentEndOverlap`
  (params (OverlappedComponent :type "PrimitiveComponent Object Reference") (OtherActor :type "Actor Object Reference") (OtherComp :type "PrimitiveComponent Object Reference") (OtherBodyIndex :type Integer))
  (cast `/Game/TopDownBP/Blueprints/PlayerCharacterBP` OtherActor)
  (set `self.IsInTrigger` false))

(event `InputAction|Interact` :consume false
  (params (Key :type "Key Structure"))
  (:`Pressed`
    (if (`self.IsInTrigger`)
      (cast `/Game/TopDownBP/Blueprints/PlayerCharacterBP` (`GameplayStatics.GetPlayerCharacter` 0))
      (bind _returnvalue (`|CreateWidget` "/Game/UI_Widgets/Pick-up_Widget/NothingHere_Widget.NothingHere_Widget_C" (`GameplayStatics.GetPlayerController` 0)))
      (`UserWidget.AddToViewport` _returnvalue 0))))

(fn `UserConstructionScript`)